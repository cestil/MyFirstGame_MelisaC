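; Game mode that keeps the player's score and declares a win once it reaches a fixed threshold.
; ScoreF adds the given enemy points to Score and prints the total through a DoOnce.
; Tick polls Score every frame and uses a DoOnce to call WinF a single time.
; Win and start feedback are only printed debug strings.
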(event EventBeginPlay
  (Development|PrintString "START"))

(event EventTick
  (params (DeltaSeconds :type Float%20%28single-precision%29))
  (if (>= (Variables|Default|GetScore) 150)
    (Utilities|FlowControl|DoOnce false
      (:Completed
        (CallFunction|WinF)))))

(fn ConstructionScript)

(fn ScoreF
  (params (Enemy%20Point :type Integer))
  (bind _output_get (Variables|Default|SetScore (+ (Variables|Default|GetScore) Enemy%20Point)))
  (Utilities|FlowControl|DoOnce false
    (:Completed
      (Development|PrintString (Utilities|String|ToString(Integer) _output_get)))))

(fn WinF
  (Development|PrintString "YOU WIN"))