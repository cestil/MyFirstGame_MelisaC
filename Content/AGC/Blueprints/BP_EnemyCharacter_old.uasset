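; BP_EnemyCharacter_old is an enemy Character that pursues the player.
; BeginPlay caches GM_GameMode, sets walk speed and starts Chase, an AIMoveTo that re-calls itself on success without passing the target.
; Capsule overlap with a "Player"-tagged actor passes Damage to the game mode's HPF.
; AnyDamage lowers CurrentHP only when IsDead is already true, and turns mesh physics simulation off at zero HP.
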(event OnComponentBeginOverlap(CapsuleComponent)
  (params (OverlappedComponent :type Primitive%20Component%20Object%20Reference) (OtherActor :type Actor%20Object%20Reference) (OtherComp :type Primitive%20Component%20Object%20Reference) (OtherBodyIndex :type Integer) (bFromSweep :type Boolean) (SweepResult :type Hit%20Result%20Structure%20%28by%20ref%29))
  (if (Actor|ActorHasTag OtherActor "Player")
    (Default|HPF (Variables|Default|GetGame%20Mode) (Variables|Default|GetDamage))))

(event Custom|Chase
  (params (TargetChase :type Actor%20Object%20Reference))
  (AI|AIMoveTo self "0, 0, 0" TargetChase 5.0 false
    (:OnSuccess
      (CallFunction|Chase) ; agar event Chase dilakukan terus-menerus
    )))

(event EventBeginPlay
  ;[1 1 1] Cast to GM
  (bind _asgm_game_mode (Utilities|Casting|CastToGM_GameMode (Game|GetGameMode)))
  (Variables|Default|SetGame%20Mode _asgm_game_mode)
  (bind _asbp_main_character (Utilities|Casting|CastToBP_MainCharacter (Game|GetPlayerCharacter 0)))
  (Variables|/Script/Engine.CharacterMovementComponent|SetMaxWalkSpeed (Variables|Character|GetCharacterMovement) 2e+02)
  (CallFunction|Chase _asbp_main_character))

(event Collision|EventActorBeginOverlap
  (params (OtherActor :type Actor%20Object%20Reference)))

(event EventTick
  (params (DeltaSeconds :type Float%20%28single-precision%29)))

(event Game|Damage|EventAnyDamage
  (params (Damage :type Float%20%28single-precision%29) (DamageType :type Damage%20Type%20Object%20Reference) (InstigatedBy :type Controller%20Object%20Reference) (DamageCauser :type Actor%20Object%20Reference))
  (if (Variables|Default|GetIsDead?)
    (bind _output_get (Variables|Default|SetCurrentHP (- (Variables|Default|GetCurrentHP) Damage)))
    (Development|PrintString (Utilities|String|ToString(Float) _output_get))
    (Variables|Default|SetIsDead? (<= (Variables|Default|GetCurrentHP) 0.0))
    (Development|PrintString "Is Dead" true true "(R=0.291667,G=0.015336,B=0.000000,A=1.000000)")
    (if (Variables|Default|GetIsDead?)
      (Physics|SetSimulatePhysics (Variables|Character|GetMesh) false))))

(fn ConstructionScript)