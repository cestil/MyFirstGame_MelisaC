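; BP_FieldHeal is a one-shot field pickup that heals the player and awards score.
; It caches the game mode and main character on BeginPlay.
; When a Player-tagged actor overlaps Enemy_collider, a DoOnce spawns a buff particle at the pickup's location and calls GetFieldHeal on the cached character.
; It then destroys itself and passes Point to the game mode's ScoreF.
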(event OnComponentBeginOverlap(Enemy_collider)
  (params (OverlappedComponent :type Primitive%20Component%20Object%20Reference) (OtherActor :type Actor%20Object%20Reference) (OtherComp :type Primitive%20Component%20Object%20Reference) (OtherBodyIndex :type Integer) (bFromSweep :type Boolean) (SweepResult :type Hit%20Result%20Structure%20%28by%20ref%29))
  (bind _returnvalue (Transformation|GetActorLocation))
  (if (Actor|ActorHasTag OtherActor "Player")
    (Utilities|FlowControl|DoOnce false
      (:Completed
        (Utilities|FlowControl|Sequence
          (:then_0
            (Effects|SpawnEmitteratLocation "/Game/InfinityBladeEffects/Effects/FX_Ability/Heal/PC_Health_Player_Buff_Ping_02.PC_Health_Player_Buff_Ping_02" (Math|Vector|MakeVector (.x _returnvalue) (.y _returnvalue) 0.0) "0, 0, 0" "1.500000,1.500000,1.000000")
            (Default|GetFieldHeal (Variables|Default|GetMain%20Character)))
          (:then_1
            (Actor|DestroyActor)
            (Default|ScoreF (Variables|Default|GetGame%20Mode) (Variables|Default|GetPoint))))))))

(event EventBeginPlay
  (bind _asgm_game_mode (Utilities|Casting|CastToGM_GameMode (Game|GetGameMode)))
  (Variables|Default|SetGame%20Mode _asgm_game_mode)
  (bind _asbp_main_character (Utilities|Casting|CastToBP_MainCharacter (Game|GetPlayerCharacter 0)))
  (Variables|Default|SetMain%20Character _asbp_main_character))

(event EventTick
  (params (DeltaSeconds :type Float%20%28single-precision%29)))

(fn ConstructionScript)