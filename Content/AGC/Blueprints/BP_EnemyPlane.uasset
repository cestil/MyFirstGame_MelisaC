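; BP_EnemyPlane is an enemy plane actor that is destroyed and awards points when the player touches it.
; On BeginPlay it caches the GM_GameMode reference.
; When Enemy_collider overlaps an actor tagged Player, it destroys itself and passes its Point value to the game mode's ScoreF.
; The construction script applies a configurable MaterialChange material to the mesh, so instances can look different.
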(event OnComponentBeginOverlap(Enemy_collider)
  (params (OverlappedComponent :type Primitive%20Component%20Object%20Reference) (OtherActor :type Actor%20Object%20Reference) (OtherComp :type Primitive%20Component%20Object%20Reference) (OtherBodyIndex :type Integer) (bFromSweep :type Boolean) (SweepResult :type Hit%20Result%20Structure%20%28by%20ref%29))
  (if (Actor|ActorHasTag OtherActor "Player")
    (Actor|DestroyActor)
    (Default|ScoreF (Variables|Default|GetGame%20Mode) (Variables|Default|GetPoint))))

(event EventBeginPlay
  (bind _asgm_game_mode (Utilities|Casting|CastToGM_GameMode (Game|GetGameMode)))
  (Variables|Default|SetGame%20Mode _asgm_game_mode))

(event EventTick
  (params (DeltaSeconds :type Float%20%28single-precision%29)))

(fn ConstructionScript
  (Rendering|Material|SetMaterial (Variables|Default|GetEnemy_mesh) 0 (Variables|Default|GetMaterial%20Change)))