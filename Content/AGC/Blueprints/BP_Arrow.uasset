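; BP_Arrow is an arrow projectile that stays collisionless until Shoot launches it.
; Shoot adds a projectile movement component at runtime, scaling speed and gravity by draw strength, then enables the collision box.
; Overlapping anything but the instigator stops and attaches the arrow, sets a lifespan, applies launch velocity as impulse to simulating bodies and prints the hit component.
; Spawn and destroy helpers look unfinished, with character assignment and socket attachment unwired.
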(event OnComponentBeginOverlap(BoxCollission)
  (params (OverlappedComponent :type Primitive%20Component%20Object%20Reference) (OtherActor :type Actor%20Object%20Reference) (OtherComp :type Primitive%20Component%20Object%20Reference) (OtherBodyIndex :type Integer) (bFromSweep :type Boolean) (SweepResult :type Hit%20Result%20Structure%20%28by%20ref%29))
  (bind _hitcomponent (Collision|BreakHitResult SweepResult))
  (if (!= OtherActor (Game|GetInstigator))
    (bind _projectilemovementcomponent (Variables|Default|GetProjectileMovementComponent)
      (:then
        (Components|DestroyComponent _projectilemovementcomponent))
      (:else
        _))
    (Collision|SetCollisionEnabled (Variables|Default|GetBoxCollission) "NoCollision")
    (Transformation|AttachComponentToComponent _hitcomponent "None" "KeepWorld" "KeepWorld" "KeepWorld" true)
    (Actor|SetLifeSpan 1e+01)
    (if (Physics|IsSimulatingPhysics _hitcomponent "None")
      (Physics|AddImpulse _hitcomponent (Variables|Default|GetVelocity_var) "None" true))
    (Development|PrintString (Utilities|GetDisplayName _hitcomponent))))

(event Custom|Shoot
  (params (Direction :type Vector) (Strength :type Float%20%28double-precision%29))
  (bind _returnvalue (AddComponent|AddProjectileMovementComponent))
  (bind _output_get (Variables|Default|SetProjectileMovementComponent _returnvalue))
  (bind _output_get_2 (Variables|/Script/Engine.MovementComponent|SetVelocity _output_get (* Direction (Math|Float|Lerp (Variables|Default|GetMinSpeed) (Variables|Default|GetMaxSpeed) Strength))))
  (Variables|Default|SetVelocity_var _output_get_2)
  (Variables|/Script/Engine.ProjectileMovementComponent|SetProjectileGravityScale _returnvalue (Math|Float|Lerp (Variables|Default|GetMaxGravity) (Variables|Default|GetMinGravity) Strength))
  (Collision|SetCollisionEnabled (Variables|Default|GetBoxCollission) "QueryAndPhysics"))

(event EventBeginPlay
  (Collision|SetCollisionEnabled (Variables|Default|GetBoxCollission) "NoCollision"))

(event Collision|EventActorBeginOverlap
  (params (OtherActor :type Actor%20Object%20Reference)))

(event EventTick
  (params (DeltaSeconds :type Float%20%28single-precision%29)))

(fn ConstructionScript)

(fn SpawnArrowF
  (Game|SpawnActorfromClass "BP_Arrow_C" (Math|Transform|MakeTransform "0, 0, 0" "0, 0, 0" "1.000000,1.000000,1.000000") "Undefined" "MultiplyWithRoot" 0 (Variables|Default|GetMainCharacter)))

(fn DestroyArrowF
  (bind _arrow_ref (Variables|Default|GetArrow_Ref)
    (:then
      (Actor|DestroyActor _arrow_ref))
    (:else)))