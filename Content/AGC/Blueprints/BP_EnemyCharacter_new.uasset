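; Sword-and-shield enemy character that chases and attacks the player once PawnSensing spots a pawn, with a camera-facing health bar.
; Chase and Attack loop through AI MoveTo, a short line trace from the sword socket applying damage, and one of two random slash montages.
; Damage triggers hit effects and an impact montage, or on death adds score and disables collision.
; Patrol and Alert events exist but are not called here.
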(event OnComponentBeginOverlap(CapsuleComponent)
  (params (OverlappedComponent :type Primitive%20Component%20Object%20Reference) (OtherActor :type Actor%20Object%20Reference) (OtherComp :type Primitive%20Component%20Object%20Reference) (OtherBodyIndex :type Integer) (bFromSweep :type Boolean) (SweepResult :type Hit%20Result%20Structure%20%28by%20ref%29)))

(event OnSeePawn(PawnSensing)
  (params (Pawn :type Pawn%20Object%20Reference))
  (Utilities|FlowControl|DoOnce false
    (:Completed
      (if (Math|Boolean|NORBoolean (Variables|Default|GetIsDead?) (Variables|/Game/AGC/Blueprints/BP_MainCharacter.BP_MainCharacter_C|GetIsDead? (Variables|Default|GetPlayerCharacter)))
        (Variables|Default|SetIsIdle? false)
        (Variables|Default|SetIsAlert? false)
        (bind _newtrack_0 (Timeline|Timeline Play)
          (:Update
            (Variables|/Script/Engine.CharacterMovementComponent|SetMaxWalkSpeed (Variables|Character|GetCharacterMovement) (Math|Float|Lerp 0.0 4e+02 _newtrack_0))
            (CallFunction|Chase (Variables|Default|GetPlayerCharacter))))))))

(event Custom|Chase
  (params (TargetChase :type Actor%20Object%20Reference))
  (if (Math|Boolean|NORBoolean (Variables|Default|GetIsDead?) (Variables|/Game/AGC/Blueprints/BP_MainCharacter.BP_MainCharacter_C|GetIsDead? (Variables|Default|GetPlayerCharacter)))
    (Variables|Default|SetIfAttack? false)
    (Development|PrintString "IS CHASING")
    (Variables|/Script/Engine.CharacterMovementComponent|SetMaxWalkSpeed (Variables|Character|GetCharacterMovement) 4e+02)
    (AI|AIMoveTo self "0, 0, 0" TargetChase 1.5e+02 false
      (:OnSuccess
        (CallFunction|Attack))
      (:OnFail
        (CallFunction|Chase (Variables|Default|GetPlayerCharacter)) ; agar event Chase dilakukan terus-menerus
      ))))

(event Custom|Patrol
  (Utilities|FlowControl|DoOnce false
    (:Completed
      (if (not (Variables|Default|GetIsDead?))
        (Variables|Default|SetIsIdle? false)
        (Variables|/Script/Engine.CharacterMovementComponent|SetMaxWalkSpeed (Variables|Character|GetCharacterMovement) 1e+02)
        (AI|AIMoveTo self (.OutItem (Utilities|Array|Random (Variables|Default|GetPatrol%20Point))) 0 0.0 false
          (:OnSuccess
            _)
          (:OnFail
            _))
        (CallFunction|Patrol) ; agar event Patrol dilakukan terus-menerus
      ))))

(event Custom|Attack
  (bind _sword (Variables|Default|GetSword))
  (bind _mesh (Variables|Character|GetMesh))
  (bind _playercharacter (Variables|Default|GetPlayerCharacter))
  (bind _returnvalue (Transformation|GetSocketTransform _sword "damage_socket" "RTS_World"))
  (if (Math|Boolean|NORBoolean (Variables|Default|GetIsDead?) (Variables|/Game/AGC/Blueprints/BP_MainCharacter.BP_MainCharacter_C|GetIsDead? (Variables|Default|GetPlayerCharacter)))
    (bind _output_get (Variables|Default|SetWhichAttack? (Math|Random|RandomIntegerinRange 0 1)))
    (Variables|Default|SetIfAttack? true)
    (Development|PrintString "IS ATTACK" true true "(R=0.734375,G=0.286254,B=0.024102,A=1.000000)")
    ;[1 1 1] Line Trace
    (bind (_outhit _returnvalue_2) (Collision|LineTraceByChannel (.location _returnvalue) (+ (.location _returnvalue) (* (Math|Vector|GetRightVector (Variables|Character|GetMesh)) 1e+02)) "TraceTypeQuery1" false 0 "None"))
    (if _returnvalue_2
      (Development|PrintString (Utilities|GetDisplayName (.HitActor (Collision|BreakHitResult _outhit)))))
    (if (== (.HitActor (Collision|BreakHitResult _outhit)) _playercharacter)
      (Game|Damage|ApplyDamage _playercharacter 2e+01 0 0)
      ;[1 1 1] Attack Animation Choices
      (switch int _output_get
        (:0
          (Animation|Montage|PlayMontage _mesh "/Game/AGC/Animations/Enemy_A/E_Attack/AM_E1_sword_and_shield_slash.AM_E1_sword_and_shield_slash"
            (:OnCompleted
              _)
            (:OnInterrupted
              _)))
        (:1
          (Animation|Montage|PlayMontage _mesh "/Game/AGC/Animations/Enemy_A/E_Attack/AM_E2_sword_and_shield_slash__3_.AM_E2_sword_and_shield_slash__3_"
            (:OnCompleted
              _)
            (:OnInterrupted
              _)))))
    (CallFunction|Chase (Variables|Default|GetPlayerCharacter)) ; Back to Chase Player
  ))

(event Custom|Alert
  (params (HitLocation :type Vector))
  (bind _returnvalue (Transformation|GetActorLocation))
  (bind _returnvalue_2 (Math|Rotator|FindLookatRotation _returnvalue HitLocation))
  (Utilities|FlowControl|Delay 0.5)
  (Transformation|SetActorRotation (Math|Rotator|MakeRotator (.roll _returnvalue_2) 0.0 (.yaw _returnvalue_2))))

(event EventBeginPlay
  ;[1 1 1] Cast to GM
  (bind _asgm_game_mode (Utilities|Casting|CastToGM_GameMode (Game|GetGameMode)))
  (Variables|Default|SetGame%20Mode _asgm_game_mode)
  ;[1 1 1] Cast to Player Character
  (bind _asbp_main_character (Utilities|Casting|CastToBP_MainCharacter (Game|GetPlayerCharacter 0)))
  (Variables|Default|SetPlayerCharacter _asbp_main_character)
  ;[1 1 1] Cast to HP Widget
  (bind _aswbp_enemy_health_bar (Utilities|Casting|CastToWBP_EnemyHealthBar (UserInterface|GetWidget (Variables|Default|GetHP_Bar))))
  (Variables|Default|Set%20WBP_HP%20Bar _aswbp_enemy_health_bar)
  ;[1 1 1] Temp State
  (Variables|Default|SetIsEquip? true)
  (Variables|Default|SetIsIdle? true)
  (Utilities|FlowControl|Delay 2.0))

(event Collision|EventActorBeginOverlap
  (params (OtherActor :type Actor%20Object%20Reference)))

(event EventTick
  (params (DeltaSeconds :type Float%20%28single-precision%29))
  (bind __wbp_hp_bar (Variables|Default|Get%20WBP_HP%20Bar))
  (Utilities|IsValid __wbp_hp_bar
    (:Is%20Valid
      (Default|HPBarF __wbp_hp_bar (Variables|Default|GetCurrentHP) (Variables|Default|GetMaxHP))
      (Transformation|SetWorldRotation (Variables|Default|GetHP_Bar) (Math|Rotator|FindLookatRotation (Transformation|GetActorLocation) (Transformation|GetActorLocation (Game|GetPlayerCameraManager 0))) false false))))

(event Game|Damage|EventAnyDamage
  (params (Damage :type Float%20%28single-precision%29) (DamageType :type Damage%20Type%20Object%20Reference) (InstigatedBy :type Controller%20Object%20Reference) (DamageCauser :type Actor%20Object%20Reference))
  (if (not (Variables|Default|GetIsDead?))
    (Audio|PlaySoundatLocation "/Game/AGC/Sounds/Bow_Arrow/ArrowHitDummy2_Cue.ArrowHitDummy2_Cue" (Transformation|GetActorLocation) "0, 0, 0" 1.0 1.0 0.0 0 0 0 0) ; SFX - Bow Hit
    (Effects|SpawnEmitterAttached "/Game/FXVarietyPack/Particles/P_ky_ThunderBallHit.P_ky_ThunderBallHit" (Variables|Character|GetMesh) "HitVFX_socket" "0, 0, 0" "0, 0, 0" "0.200000,0.200000,0.200000")
    (bind _output_get (Variables|Default|SetCurrentHP (- (Variables|Default|GetCurrentHP) Damage)))
    (Development|PrintString (Utilities|String|ToString(Float) _output_get) true true "(R=0.643582,G=0.014323,B=0.687500,A=1.000000)")
    (if (<= (Variables|Default|GetCurrentHP) 0.0)
      (Variables|Default|SetIsAlert? false)
      (Variables|Default|SetIsDead? (<= (Variables|Default|GetCurrentHP) 0.0))
      (Default|ScoreFNew (Variables|Default|GetGame%20Mode) 1.0)
      (Development|PrintString "Is Dead" true true "(R=0.291667,G=0.015336,B=0.000000,A=1.000000)")
      (Collision|SetCollisionEnabled (Variables|Character|GetMesh) "NoCollision")
      (Development|SetHiddeninGame (Variables|Default|GetHP_Bar) true false)
      (else
        (Variables|Default|SetIsHit? true)
        ;[1 1 1] Old
        (Animation|Montage|PlayMontage (Variables|Character|GetMesh) "/Game/AGC/Animations/Enemy_A/F_Hit/AM_F1_sword_and_shield_impact__2_.AM_F1_sword_and_shield_impact__2_"
          (:OnCompleted
            _)
          (:OnInterrupted
            _))
        (Variables|Default|SetIsHit? false)
        (if (Variables|Default|GetIsIdle?)
          (Variables|Default|SetIsAlert? false))
        (Utilities|FlowControl|Delay 5.0)))))

(fn ConstructionScript)

(fn AlertF
  (params (HitLocation :type Vector))
  (bind _returnvalue (Transformation|GetActorLocation))
  (bind _returnvalue_2 (Math|Rotator|FindLookatRotation _returnvalue HitLocation))
  (Transformation|SetActorRotation (Math|Rotator|MakeRotator (.roll _returnvalue_2) 0.0 (.yaw _returnvalue_2))))