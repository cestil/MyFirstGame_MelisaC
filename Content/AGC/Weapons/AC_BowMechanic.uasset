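; AC_BowMechanic is an actor component that gives its owning Character bow-and-arrow shooting.
; Its functions spawn the bow and a BP_Arrow onto mesh sockets and can destroy the arrow.
; BeginDraw starts a looping timer that accumulates draw time, and EndDraw clears it.
; BeginShoot detaches the arrow, fires it along the camera's forward vector with draw time normalized and clamped as strength, then ends the draw.
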(event Custom|BeginShoot
  (bind _arrow_ref (Variables|Default|GetArrow_Ref)
    (:then
      (Transformation|DetachFromActor _arrow_ref "KeepWorld" "KeepWorld" "KeepWorld")
      (Default|Shoot _arrow_ref (Math|Vector|GetForwardVector (Actor|GetComponentbyClass (Variables|Default|GetCharacter_Ref) "/Script/Engine.CameraComponent")) (Math|Float|Clamp(Float) (Math|Float|NormalizetoRange (Variables|Default|GetDrawDuration) 0.0 (Variables|Default|GetMaxDrawDuration))))
      (CallFunction|EndDraw))
    (:else)))

(event Custom|BeginDraw
  (bind _returnvalue (Utilities|Time|SetTimerbyEvent (delegate Custom|IncrementDrawTime) (Variables|Default|GetDrawIncrementTime) true))
  (Variables|Default|SetDrawTimer _returnvalue))

(event Custom|IncrementDrawTime
  (bind _output_get (Variables|Default|SetDrawDuration (+ (Variables|Default|GetDrawDuration) (Variables|Default|GetDrawIncrementTime)))))

(event Custom|EndDraw
  (Variables|Default|SetDrawDuration 0.0)
  (Utilities|Time|ClearandInvalidateTimerbyHandle (Variables|Default|GetDrawTimer)))

(event EventBeginPlay
  (bind _ascharacter (Utilities|Casting|CastToCharacter (Components|GetOwner)))
  (Variables|Default|SetCharacter_Ref _ascharacter))

(event EventTick
  (params (DeltaSeconds :type Float%20%28single-precision%29)))

(fn EquipF
  (bind _returnvalue (Game|SpawnActorfromClass (Variables|Default|GetBowClass) (Math|Transform|MakeTransform "0, 0, 0" "0, 0, 0" "1.000000,1.000000,1.000000") "Undefined" "MultiplyWithRoot" 0 0))
  (Transformation|AttachComponentToComponent _returnvalue (Variables|/Script/Engine.Character|GetMesh (Variables|Default|GetCharacter_Ref)) (Variables|Default|GetBowSocketName) "SnapToTarget" "SnapToTarget" "SnapToTarget" true))

(fn SpawnArrowF
  (bind _returnvalue (Game|SpawnActorfromClass "/Game/AGC/Blueprints/BP_Arrow.BP_Arrow_C" (Math|Transform|MakeTransform "0, 0, 0" "0, 0, 0" "1.000000,1.000000,1.000000") "Undefined" "MultiplyWithRoot" 0 (Variables|Default|GetCharacter_Ref)))
  (bind _output_get (Variables|Default|SetArrow_Ref _returnvalue))
  (Transformation|AttachComponentToComponent _output_get (Variables|/Script/Engine.Character|GetMesh (Variables|Default|GetCharacter_Ref)) (Variables|Default|GetArrowSocket%20Name) "SnapToTarget" "SnapToTarget" "SnapToTarget" true))

(fn DestroyArrowF
  (bind _arrow_ref (Variables|Default|GetArrow_Ref)
    (:then
      (Actor|DestroyActor _arrow_ref))
    (:else)))