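; Actor component that gives its owning Character a bow and arrows, despite its enemy sword mechanic name.
; BeginPlay caches the owner as a Character, whose mesh serves as the attach point for spawned weapons.
; EquipF spawns the bow class onto a socket, and SpawnArrowF spawns, stores and attaches a BP_Arrow instigated by that Character.
; Neither function is called within the component, as the EquipF call in the event graph is unwired.
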(event EventBeginPlay
  (bind _ascharacter (Utilities|Casting|CastToCharacter (Components|GetOwner)))
  (Variables|Default|SetCharacter_Ref _ascharacter))

(event EventTick
  (params (DeltaSeconds :type Float%20%28single-precision%29)))

(fn EquipF
  (bind _returnvalue (Game|SpawnActorfromClass (Variables|Default|GetBowClass) (Math|Transform|MakeTransform "0, 0, 0" "0, 0, 0" "1.000000,1.000000,1.000000") "Undefined" "MultiplyWithRoot" 0 0))
  (Transformation|AttachComponentToComponent _returnvalue (Variables|/Script/Engine.Character|GetMesh (Variables|Default|GetCharacter_Ref)) (Variables|Default|GetBowSocketName) "SnapToTarget" "SnapToTarget" "SnapToTarget" true))

(fn SpawnArrowF
  (bind _returnvalue (Game|SpawnActorfromClass "/Game/AGC/Blueprints/BP_Arrow.BP_Arrow_C" (Math|Transform|MakeTransform "0, 0, 0" "0, 0, 0" "1.000000,1.000000,1.000000") "Undefined" "MultiplyWithRoot" 0 (Variables|Default|GetCharacter_Ref)))
  (bind _output_get (Variables|Default|SetArrow_Ref _returnvalue))
  (Transformation|AttachComponentToComponent _output_get (Variables|/Script/Engine.Character|GetMesh (Variables|Default|GetCharacter_Ref)) (Variables|Default|GetArrowSocket%20Name) "SnapToTarget" "SnapToTarget" "SnapToTarget" true))